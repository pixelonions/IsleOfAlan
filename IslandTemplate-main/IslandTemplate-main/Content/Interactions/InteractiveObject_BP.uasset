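; Interactive object Blueprint that shows an interact icon prompt when highlighted.
; On BeginPlay it creates an InteractIcon widget and assigns it to its Widget component.
; Highlight makes the component visible and sets the icon from the IslandGame_PC player controller's UseGamepadUI flag, while DeHighlight hides it.
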(event `self.ReceiveBeginPlay`
  (bind _returnvalue (`|CreateWidget` "/Game/Characters/UI/InteractIcon.InteractIcon_C"))
  (bind _output_get (set `self.InteractIcon` _returnvalue))
  (`WidgetComponent.SetWidget` (`self.Widget`) _output_get))

(event `/Game/Game/InteractionInterface.Highlight`
  (bind _widget (`self.Widget`))
  (`/Engine/EditorBlueprintResources/StandardMacros.IsValid` _widget
    (:`Is Valid`
      (`SceneComponent.SetVisibility` _widget true false)
      (`/Game/Characters/UI/InteractIcon.SetIconToUse` (`self.InteractIcon`) (`/Game/Game/IslandGame_PC.UseGamepadUI` (cast `/Game/Game/IslandGame_PC` (`GameplayStatics.GetPlayerController` 0) :!pure true))))))

(event `/Game/Game/InteractionInterface.DeHighlight`
  (bind _widget (`self.Widget`))
  (`/Engine/EditorBlueprintResources/StandardMacros.IsValid` _widget
    (:`Is Valid`
      (`SceneComponent.SetVisibility` _widget false false))))

(fn `UserConstructionScript`)