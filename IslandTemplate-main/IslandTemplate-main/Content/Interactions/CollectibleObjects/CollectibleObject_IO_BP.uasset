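; Interactable collectible actor that the player picks up, adding it to the controller's inventory and setting a gameplay tag on the game instance.
; Interact shows a name and description widget, then either removes the item after a short delay or, with DoCollectionCamera, attaches it to the character's display socket with a montage and camera-state change.
; Continue plays the montage's exit, restores the camera and destroys the actor.
; The construction script stamps the actor's own class into its inventory data.
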(event `/Game/Game/InteractionInterface.Interact`
  (params (InstigatingCharacter :type "/Game/Characters/IslandCharacter_C Object Reference") (`AI Interact Task` :type "/Game/Characters/NPC/AI/Tasks/Interact_Task Object Reference"))
  (bind (_inventoryobjectdata_objectname _inventoryobjectdata_objectdescription) (break `/Game/Interactions/CollectibleObjects/Inventory/InventoryObjectData` (`self.InventoryObjectData`)))
  (bind _playercharacter (`self.PlayerCharacter`))
  (bind _asplayer_island_character_c (cast `/Game/Characters/Player/Player_IslandCharacter_C` InstigatingCharacter))
  (bind _output_get (set `self.PlayerCharacter` _asplayer_island_character_c))
  (bind _asisland_game_instance_gi (cast `/Game/Game/IslandGameInstance_GI` (`GameplayStatics.GetGameInstance`)))
  (`BlueprintGameplayTagLibrary.AddGameplayTag` (`/Game/Game/IslandGameInstance_GI.IslandGameplayTags` _asisland_game_instance_gi) (`self.TagToSet`))
  (bind _asisland_game_pc (cast `/Game/Game/IslandGame_PC` (`Pawn.GetController` _output_get)))
  (set `self.IslandGamePC` _asisland_game_pc)
  (`|ExecutionSequence`
    (:`then_0`
      ; Show Collectible Widget
      (bind _returnvalue (`|CreateWidget` "/Game/Interactions/CollectibleObjects/CollectibleObjectWidget_W.CollectibleObjectWidget_W_C" null (`KismetTextLibrary.Conv_TextToString` _inventoryobjectdata_objectname) (`KismetTextLibrary.Conv_TextToString` _inventoryobjectdata_objectdescription)))
      (bind _output_get_2 (set `self.CollectedWidget` _returnvalue))
      (`UserWidget.AddToViewport` _output_get_2 0))
    (:`then_1`
      (if (`self.DoCollectionCamera`)
        ; Collection Camera
        (set `/Game/Game/IslandGame_PC.CurrentInteractionActor` self _asisland_game_pc)
        (`PrimitiveComponent.SetCollisionEnabled` (`self.Mesh`) "NoCollision")
        (`self.K2_AttachToComponent` (`Character.Mesh` _playercharacter) "ObjectDisplayPoint" "SnapToTarget" "SnapToTarget" "KeepWorld" false)
        (set `/Game/Characters/Player/Player_IslandCharacter_C.CurrentCameraState` "NewEnumerator2" _playercharacter)
        (`|PlayMontage` (`Character.Mesh` _playercharacter) "/Game/Characters/Animation/Collectible_Montage.Collectible_Montage" 1.0 0.0 "Default")))
    (:`then_2`
      ; Add Object To Inventory
      (`/Game/Interactions/CollectibleObjects/Inventory/Inventory_C.AddObject` (`/Game/Game/IslandGame_PC.Inventory_C` _asisland_game_pc) (`self.InventoryObjectData`))
      ; Remove Widget After Time Elapsed (if not doing collection camera)
      (if (not (`self.DoCollectionCamera`))
        (`ActorComponent.K2_DestroyComponent` (`self.Widget`))
        (`ActorComponent.K2_DestroyComponent` (`self.Mesh`))
        (`KismetSystemLibrary.Delay` 1.0)
        (`Widget.RemoveFromParent` (`self.CollectedWidget`))
        (`self.K2_DestroyActor`)))))

(event `/Game/Game/InteractionInterface.Continue`
  (bind _islandgamepc (`self.IslandGamePC`))
  (bind _returnvalue (`Controller.K2_GetPawn` _islandgamepc))
  (if (`self.DoCollectionCamera`)
    (`|PlayMontage` (`self.GetComponentByClass` _returnvalue "/Script/Engine.SkeletalMeshComponent") "/Game/Characters/Animation/Collectible_Montage.Collectible_Montage" 1.0 0.0 "Out"
      (:`then`
        (`PlayerController.SetViewTargetWithBlend` _islandgamepc _returnvalue 0.25 "VTBlend_Linear" 0.0 false)
        (`Widget.RemoveFromParent` (`self.CollectedWidget`))
        (set `/Game/Characters/Player/Player_IslandCharacter_C.CurrentCameraState` "NewEnumerator0" (`self.PlayerCharacter`))
        (`self.K2_DestroyActor`)))))

(fn `UserConstructionScript`
  (bind (_inventoryobjectdata_objectname _inventoryobjectdata_objectdescription _inventoryobjectdata_collectibleobjectclass _inventoryobjectdata_objectthumbnail _inventoryobjectdata_menuoptions) (break `/Game/Interactions/CollectibleObjects/Inventory/InventoryObjectData` (`self.InventoryObjectData`)))
  (`parent.UserConstructionScript`)
  (set `self.InventoryObjectData` (make `/Game/Interactions/CollectibleObjects/Inventory/InventoryObjectData` _inventoryobjectdata_objectname _inventoryobjectdata_objectdescription (`GameplayStatics.GetObjectClass` self) _inventoryobjectdata_objectthumbnail _inventoryobjectdata_menuoptions)))