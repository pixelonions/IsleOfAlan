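; RecolourableHat_EO_BP is a hat actor, filed under collectible cap objects, whose colour comes from a CapColour value.
; The construction script creates two dynamic material instances and sets their Colour parameter, giving mesh slot 0 the full colour and slot 1 a half-brightness shade.
; The event graph holds only disabled default events, so this Blueprint adds no runtime logic of its own.
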(fn `UserConstructionScript`
  (bind _capcolour (`self.CapColour`))
  (`parent.UserConstructionScript`)
  (bind _returnvalue (`KismetMaterialLibrary.CreateDynamicMaterialInstance` "/Game/Interactions/CollectibleObjects/Cap/Mat/CapColour.CapColour"))
  (`MaterialInstanceDynamic.SetVectorParameterValue` _returnvalue "Colour" _capcolour)
  (`PrimitiveComponent.SetMaterial` (`self.Mesh`) 0 _returnvalue)
  (bind _returnvalue_2 (`KismetMaterialLibrary.CreateDynamicMaterialInstance` "/Game/Interactions/CollectibleObjects/Cap/Mat/CapColour.CapColour"))
  (`MaterialInstanceDynamic.SetVectorParameterValue` _returnvalue_2 "Colour" (* _capcolour (`KismetMathLibrary.MakeColor` 0.5 0.5 0.5)))
  (`PrimitiveComponent.SetMaterial` (`self.Mesh`) 1 _returnvalue_2))