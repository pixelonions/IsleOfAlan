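; Interaction station that plays a level sequence when a character interacts with it.
; On BeginPlay it creates a sequence player from its configured sequence and settings and caches the resulting actor.
; Interact starts playback and Continue stops it, each after calling the parent station's logic.
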(event `self.ReceiveBeginPlay`
  (`parent.ReceiveBeginPlay`)
  (bind _outactor (`LevelSequencePlayer.CreateLevelSequencePlayer` (`self.SequenceToPlay`) (`self.SequenceSettings`)))
  (set `self.SequencePlayerActor` _outactor))

(event `/Game/Game/InteractionInterface.Interact`
  (params (InstigatingCharacter :type "/Game/Characters/IslandCharacter_C Object Reference") (`AI Interact Task` :type "/Game/Characters/NPC/AI/Tasks/Interact_Task Object Reference"))
  (`parent.Interact` InstigatingCharacter `AI Interact Task`)
  (`MovieSceneSequencePlayer.Play` (`LevelSequenceActor.SequencePlayer` (`self.SequencePlayerActor`))))

(event `/Game/Game/InteractionInterface.Continue`
  (`parent.Continue`)
  (`MovieSceneSequencePlayer.Stop` (`LevelSequenceActor.SequencePlayer` (`self.SequencePlayerActor`))))

(fn `UserConstructionScript`
  (`parent.UserConstructionScript`))